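; BPC_DroppedLoot is a child actor Blueprint for dropped loot that carries an inventory.
; Its construction script runs the parent's, then copies the content of InventoryToMake into the ACInventorySystem component.
; An unconnected loop that would fill slots with Coins stacks never runs.
; The event graph holds only disabled placeholder events, so this Blueprint adds no runtime event logic of its own.
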(fn `UserConstructionScript`
  (locals (LootAmount :type Integer))
  (`parent.UserConstructionScript`)
  (set `/Game/Blueprints/Inventory/AC_InventorySystem.Content` (`/Game/Blueprints/Inventory/AC_InventorySystem.Content` (`self.InventoryToMake`)) (`self.AC_InventorySystem`)))