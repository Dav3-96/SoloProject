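; Inventory actor component that currently only detects interactable actors near its owner; the add, remove and ground-item functions are empty stubs.
; A looping timer runs a zero-length sphere trace at the owner's location, caching the hit actor as InteractiveActor.
; It calls LookAtMessage on new hits, printing the result, and StopLookAtMessage when the trace finds nothing.
; Server_Interact is empty, with its AC_ItemData interaction logic left disconnected.
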(event `self.ReceiveTick`
  (params (DeltaSeconds :type "Float (single-precision)")))

(event `self.ReceiveBeginPlay`
  (`KismetSystemLibrary.K2_SetTimerDelegate` (delegate `TraceForItems`) 0.1 true))

(event `TraceForItems`
  (`self.InteractionTrace`))

(event `InputAction|Interact`
  (params (Key :type "Key Structure")))

(event `Server_Interact`
  (params (Target :type "Actor Object Reference")))

(fn `AddToInventory`)

(fn `CheckGroundItems`)

(fn `InteractionTrace`
  (bind _returnvalue (`Actor.K2_GetActorLocation` (`self.GetOwner`)))
  (bind (_outhit _returnvalue_2) (`KismetSystemLibrary.SphereTraceSingle` _returnvalue _returnvalue (`self.InteractionRange`) "TraceTypeQuery3" false (`|MakeArray` (`self.GetOwner`)) "None" true (struct :`R` 1.0 :`A` 1.0) (struct :`G` 1.0 :`A` 1.0) 2.0))
  (if _returnvalue_2
    (bind (_bblockinghit _binitialoverlap _time _distance _location _impactpoint _normal _impactnormal _physmat _hitactor) (`GameplayStatics.BreakHitResult` _outhit))
    (if (!= _hitactor (`self.InteractiveActor`))
      (set `self.InteractiveActor` _hitactor)
      (bind _interactiveactor (`self.InteractiveActor`)
        (:`then`
          (bind _message (message `/Game/Blueprints/Inventory/I_InteractInterface.LookAt` _interactiveactor _interactiveactor))
          (`KismetSystemLibrary.PrintString` (`KismetTextLibrary.Conv_TextToString` _message)))
        (:`else`))
      (else
        (bind _interactiveactor_2 (`self.InteractiveActor`)
          (:`then`)
          (:`else`
            (message `/Game/Blueprints/Inventory/I_InteractInterface.StopLookAt` _interactiveactor_2 _interactiveactor_2)))))
    (else
      (bind _interactiveactor_3 (`self.InteractiveActor`)
        (:`then`
          (message `/Game/Blueprints/Inventory/I_InteractInterface.StopLookAt` _interactiveactor_3 _interactiveactor_3)
          (set `self.InteractiveActor` null))
        (:`else`)))))

(fn `RemoveFromInventory`)