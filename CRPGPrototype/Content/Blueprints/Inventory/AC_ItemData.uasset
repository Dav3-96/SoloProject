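; Item data component for world items that handles picking them up into the player's inventory.
; Interactwith adds ItemID and Quantity to ACInventorySystem1; on success it loops the game mode's ground-loot slots, removing every one and destroying the actor inside that loop.
; RemovefromLootWindow clears the same kind of slots through the owning BP_TestItem's GameUI.
; LookAt and StopLookAt are empty stubs.
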(event `self.ReceiveBeginPlay`)

(event `/Game/Blueprints/Inventory/I_InteractInterface.InteractWith`
  (params (Actor :type "Actor Object Reference") (PlayerCharacter :type "/Game/Blueprints/PC_Character Object Reference"))
  (bind _ac_inventorysystem1 (`/Game/Blueprints/PC_Character.AC_InventorySystem1` PlayerCharacter))
  (bind (_itemid_datatable _itemid_rowname) (break `DataTableRowHandle` (`self.ItemID`)))
  (set `self.InteractedActor` Actor)
  (`/Engine/EditorBlueprintResources/StandardMacros.IsValid` _ac_inventorysystem1
    (:`Is Valid`
      (bind _success (`/Game/Blueprints/Inventory/AC_InventorySystem.AddToInventory` _ac_inventorysystem1 _itemid_rowname (`self.Quantity`)))
      (if _success
        (for _array_element (`self.GetUI`)
          (bind _asinventory_ground_loot_slot (cast `/Game/Blueprints/UI/Inventory/Inventory_GroundLootSlot` _array_element))
          (`Widget.RemoveFromParent` _asinventory_ground_loot_slot)
          (`Widget.RemoveFromParent` _array_element)
          (bind _interactedactor (`self.InteractedActor`)
            (:`then`
              (`Actor.K2_DestroyActor` _interactedactor))
            (:`else`)))))))

(event `/Game/Blueprints/Inventory/I_InteractInterface.RemoveFromLootWindow`
  (for _array_element (`PanelWidget.GetAllChildren` (`/Game/Blueprints/UI/Inventory/Inventory_GroundLoot.LootDisplayBox` (`/Game/Blueprints/UI/CoreGame_UI.Inventory_GroundLoot` (`/Game/Blueprints/Inventory/Items/BP_TestItem.GameUI` (cast `/Game/Blueprints/Inventory/Items/BP_TestItem` (`self.GetOwner`) :!pure true)))))
    (bind _asinventory_ground_loot_slot (cast `/Game/Blueprints/UI/Inventory/Inventory_GroundLootSlot` _array_element))
    (`Widget.RemoveFromParent` _asinventory_ground_loot_slot)))

(fn `GetUI`
  (returns (ReturnValue :type "Array of Widget Object Reference"))
  (return (`PanelWidget.GetAllChildren` (`/Game/Blueprints/UI/Inventory/Inventory_GroundLoot.LootDisplayBox` (`/Game/Blueprints/UI/CoreGame_UI.Inventory_GroundLoot` (`/Game/Blueprints/Base_GM.InGameUI` (cast `/Game/Blueprints/Base_GM` (`GameplayStatics.GetGameMode`) :!pure true)))))))

(fn `LookAt`
  (params (Actor :type "Actor Object Reference"))
  (returns (Message :type Text))
  (return ""))

(fn `StopLookAt`
  (params (Actor :type "Actor Object Reference"))
  (returns (Message :type Text))
  (return ""))