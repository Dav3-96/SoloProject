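; Clickable chest actor that pauses the game and shows its inventory in the player's in-game container UI.
; An interact radius sets CanOpen while PC_Character is inside, and a click within range passes ACInventorySystem to the UI through BP_PlayerController.
; The construction script sets a custom depth stencil on body and lid.
; LookAt, StopLookAt and OpenContainer are empty, and the deferred open via WasClicked is unconnected.
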(event `OpenContainer`)

(event `/Game/Blueprints/Inventory/I_InteractInterface.InteractWith`
  (params (Actor :type "Actor Object Reference") (PlayerCharacter :type "/Game/Blueprints/PC_Character Object Reference"))
  (bind _asbp_player_controller (cast `/Game/Blueprints/BP_PlayerController` (`GameplayStatics.GetPlayerController` 0)))
  (`/Game/Blueprints/BP_PlayerController.UIPauseGame` _asbp_player_controller)
  (`/Game/Blueprints/UI/CoreGame_UI.ShowContainer` (`/Game/Blueprints/BP_PlayerController.InGameUI` _asbp_player_controller) (`self.AC_InventorySystem`)))

(event `self.ClickCollision.OnClicked`
  (params (TouchedComponent :type "PrimitiveComponent Object Reference") (ButtonPressed :type "Key Structure"))
  (set `self.WasClicked` true)
  (if (`self.CanOpen`)
    (`/Game/Blueprints/Inventory/I_InteractInterface.InteractWith` null)))

(event `self.InteractRadius.OnComponentBeginOverlap`
  (params (OverlappedComponent :type "PrimitiveComponent Object Reference") (OtherActor :type "Actor Object Reference") (OtherComp :type "PrimitiveComponent Object Reference") (OtherBodyIndex :type Integer) (bFromSweep :type Boolean) (SweepResult :type "HitResult Structure (by ref)"))
  (cast `/Game/Blueprints/PC_Character` OtherActor)
  (set `self.CanOpen` true))

(event `self.InteractRadius.OnComponentEndOverlap`
  (params (OverlappedComponent :type "PrimitiveComponent Object Reference") (OtherActor :type "Actor Object Reference") (OtherComp :type "PrimitiveComponent Object Reference") (OtherBodyIndex :type Integer))
  (cast `/Game/Blueprints/PC_Character` OtherActor)
  (set `self.CanOpen` false)
  (set `self.WasClicked` false))

(fn `LookAt`
  (params (Actor :type "Actor Object Reference"))
  (returns (Message :type Text))
  (return ""))

(fn `StopLookAt`
  (params (Actor :type "Actor Object Reference"))
  (returns (Message :type Text))
  (return ""))

(fn `UserConstructionScript`
  (`PrimitiveComponent.SetCustomDepthStencilValue` (`self.ChestBody`) 4)
  (`PrimitiveComponent.SetCustomDepthStencilValue` (`self.ChestLid`) 4))