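; BP_TestItem is a test inventory item that shows itself in the ground loot UI when looked at.
; LookAt reads the item's data table row through ACItemData, creates loot buttons via the game mode's InGameUI and returns a pickup prompt; StopLookAt removes them.
; Construction sets the mesh's custom depth stencil value from DepthColour.
; Interactwith is empty, and the button-press removal and destroy logic is disconnected.
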(event `self.ReceiveBeginPlay`
  (bind _asbase_gm (cast `/Game/Blueprints/Base_GM` (`GameplayStatics.GetGameMode`)))
  (bind _output_get (set `self.GameUI` (`/Game/Blueprints/Base_GM.InGameUI` _asbase_gm)))
  (`KismetSystemLibrary.PrintString` (`KismetSystemLibrary.GetDisplayName` _output_get)))

(event `/Game/Blueprints/Inventory/I_InteractInterface.InteractWith`
  (params (Actor :type "Actor Object Reference")))

(fn `LookAt`
  (params (Actor :type "Actor Object Reference"))
  (returns (Message :type Text))
  (bind (_itemid_datatable _itemid_rowname) (break `DataTableRowHandle` (`/Game/Blueprints/Inventory/AC_ItemData.ItemID` (`self.AC_ItemData`))))
  (bind _returnvalue (`|GetDataTableRow` _itemid_datatable _itemid_rowname)
    (:`then`
      (bind (_name _description _thumbnail _itemclass _stacksize) (break `/Game/Blueprints/Inventory/S_ItemStruct` _returnvalue))
      (`/Game/Blueprints/UI/Inventory/Inventory_GroundLoot.CreateLootButtons` (`/Game/Blueprints/UI/CoreGame_UI.Inventory_GroundLoot` (`/Game/Blueprints/Base_GM.InGameUI` (cast `/Game/Blueprints/Base_GM` (`GameplayStatics.GetGameMode`) :!pure true))) _name _thumbnail _stacksize Actor)
      (return (`|FormatText` "Pickup {item}" _name)))))

(fn `StopLookAt`
  (params (Actor :type "Actor Object Reference"))
  (returns (Message :type Text))
  (`/Game/Blueprints/UI/Inventory/Inventory_GroundLoot.RemoveLootButtons` (`/Game/Blueprints/UI/CoreGame_UI.Inventory_GroundLoot` (`/Game/Blueprints/Base_GM.InGameUI` (cast `/Game/Blueprints/Base_GM` (`GameplayStatics.GetGameMode`) :!pure true))))
  (return ""))

(fn `UserConstructionScript`
  (`PrimitiveComponent.SetCustomDepthStencilValue` (`self.Mesh`) (`self.DepthColour`)))