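; Tutorial chest Blueprint that stocks its inventory with starter gear matching the player's class.
; On BeginPlay, SetupClassItems reads the Class value from the Master_Instance game instance and switches across Fighter, Ranger, Thief, Cleric, Druid and Wizard.
; Each branch writes that class's starter item into the ACInventorySystem Content array.
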(event `self.ReceiveBeginPlay`
  (`self.SetupClassItems`))

(fn `SetupClassItems`
  (switch `int` (`/Game/Blueprints/Character_Info/Master_Instance.Class` (cast `/Game/Blueprints/Character_Info/Master_Instance` (`GameplayStatics.GetGameInstance`) :!pure true))
    (:`0`
      (`KismetArrayLibrary.Array_Set` (`/Game/Blueprints/Inventory/AC_InventorySystem.Content` (`self.AC_InventorySystem`)) 0 (`self.FighterStarter`)))
    (:`1`
      (`KismetArrayLibrary.Array_Set` (`/Game/Blueprints/Inventory/AC_InventorySystem.Content` (`self.AC_InventorySystem`)) 0 (`self.RangerStarter`)))
    (:`2`
      (`KismetArrayLibrary.Array_Set` (`/Game/Blueprints/Inventory/AC_InventorySystem.Content` (`self.AC_InventorySystem`)) 0 (`self.ThiefStarter`)))
    (:`3`
      (`KismetArrayLibrary.Array_Set` (`/Game/Blueprints/Inventory/AC_InventorySystem.Content` (`self.AC_InventorySystem`)) 0 (`self.ClericStarter`)))
    (:`4`
      (`KismetArrayLibrary.Array_Set` (`/Game/Blueprints/Inventory/AC_InventorySystem.Content` (`self.AC_InventorySystem`)) 0 (`self.DruidStarter`)))
    (:`5`
      (`KismetArrayLibrary.Array_Set` (`/Game/Blueprints/Inventory/AC_InventorySystem.Content` (`self.AC_InventorySystem`)) 0 (`self.WizardStarter`)))))

(fn `UserConstructionScript`
  (`parent.UserConstructionScript`))