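; Door actor meant to swing between Open and Closed rotations when interacted with or clicked.
; BeginPlay saves the mesh rotation as Closed and detaches the trigger box, whose overlap binds OpenCloseDoor to BP_PlayerController's interact event.
; Mesh click, mesh release and box click also call it.
; The door snaps via SetActorRotation by IsItOpen, but each branch rewrites the same flag value, so the state never toggles.
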(event `self.ReceiveBeginPlay`
  (`parent.ReceiveBeginPlay`)
  (set `self.Closed` (`SceneComponent.K2_GetComponentRotation` (`self.StaticMesh`)))
  (`SceneComponent.K2_DetachFromComponent` (`self.Box`) "KeepWorld" "KeepWorld" "KeepWorld" true))

(event `self.Box.OnComponentBeginOverlap`
  (params (OverlappedComponent :type "PrimitiveComponent Object Reference") (OtherActor :type "Actor Object Reference") (OtherComp :type "PrimitiveComponent Object Reference") (OtherBodyIndex :type Integer) (bFromSweep :type Boolean) (SweepResult :type "HitResult Structure (by ref)"))
  (bind _asbp_player_controller (cast `/Game/Blueprints/BP_PlayerController` OtherActor))
  (add `/Game/Blueprints/BP_PlayerController.Interact` _asbp_player_controller (delegate `Open/CloseDoor`)))

(event `Open/CloseDoor`
  (params (NPCLocation :type "Vector Structure"))
  (if (`self.IsItOpen?`)
    (`self.K2_SetActorRotation` (`self.Open`))
    (set `self.IsItOpen?` true)
    (else
      (`self.K2_SetActorRotation` (`self.Closed`))
      (set `self.IsItOpen?` false))))

(event `self.ReceiveTick`
  (params (DeltaSeconds :type "Float (single-precision)")))

(event `self.StaticMesh.OnClicked`
  (params (TouchedComponent :type "PrimitiveComponent Object Reference") (ButtonPressed :type "Key Structure"))
  (`self.Open/CloseDoor` :!label _label))

(event `self.StaticMesh.OnReleased`
  (params (TouchedComponent :type "PrimitiveComponent Object Reference") (ButtonReleased :type "Key Structure"))
  (goto _label))

(event `self.Box.OnClicked`
  (params (TouchedComponent :type "PrimitiveComponent Object Reference") (ButtonPressed :type "Key Structure"))
  (goto _label))

(fn `UserConstructionScript`
  (`parent.UserConstructionScript`))