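; NPC actor that the player can hover and click to start dialogue.
; On BeginPlay it links its floating nameplate widget and loads NPC lines, plus player replies if it has responses, from data tables into conversation structs.
; Hovering the capsule swaps the player controller's cursor and shows the nameplate, while clicking broadcasts itself to every NPC_Interaction implementer through an interface message.
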(event `self.CapsuleComponent.OnBeginCursorOver`
  (params (TouchedComponent :type "PrimitiveComponent Object Reference"))
  (set `PlayerController.CurrentMouseCursor` "GrabHand" (cast `/Game/Blueprints/BP_PlayerController` (`GameplayStatics.GetPlayerController` 0) :!pure true))
  ;[1 1 1] Rough
  (`SceneComponent.SetVisibility` (`self.Nameplate`) true false))

(event `self.CapsuleComponent.OnEndCursorOver`
  (params (TouchedComponent :type "PrimitiveComponent Object Reference"))
  (set `PlayerController.CurrentMouseCursor` "Default" (cast `/Game/Blueprints/BP_PlayerController` (`GameplayStatics.GetPlayerController` 0) :!pure true))
  ;[1 1 1] Rough
  (`SceneComponent.SetVisibility` (`self.Nameplate`) false false))

(event `self.ReceiveBeginPlay`
  (bind _returnvalue (`GameplayStatics.GetPlayerController` 0))
  (set `/Game/Blueprints/UI/FloatingNames/FloatingNames.NPC` self (cast `/Game/Blueprints/UI/FloatingNames/FloatingNames` (`WidgetComponent.GetWidget` (`self.Nameplate`)) :!pure true))
  (set `self.As BP Player Controller` (cast `/Game/Blueprints/BP_PlayerController` _returnvalue :!pure true))
  (set `self.PlayerCharacter` (cast `/Game/Blueprints/BaseChar_BP` (`Controller.K2_GetPawn` _returnvalue) :!pure true))
  (bind _outrownames (`DataTableFunctionLibrary.GetDataTableRowNames` (`self.NPC_SpeechTable`)))
  (for _array_element _outrownames
    (bind _returnvalue_2 (`|GetDataTableRow` (`self.NPC_SpeechTable`) _array_element)
      (:`then`
        (`KismetArrayLibrary.Array_Add` (`self.TempDialogueArray`) _returnvalue_2))))
  (setmembers `/Game/Blueprints/Dialogues_OLD/NPC_TotalConveration` :`StructRef` (`self.NPC_Conversations`) :`Dialogue` (`self.TempDialogueArray`))
  (if (`self.Has Responses?`)
    (bind _outrownames_2 (`DataTableFunctionLibrary.GetDataTableRowNames` (`self.PlayerSpeechReplies`)))
    (for _array_element_2 _outrownames_2
      (bind _returnvalue_3 (`|GetDataTableRow` (`self.PlayerSpeechReplies`) _array_element_2)
        (:`then`
          (`KismetArrayLibrary.Array_Add` (`self.TempPlayerRepsonse`) _returnvalue_3))))
    (setmembers `/Game/Blueprints/Dialogues_OLD/Player_TotalConversation` :`StructRef` (`self.Player_Responses`) :`Dialogue` (`self.TempPlayerRepsonse`))))

(event `self.CapsuleComponent.OnClicked`
  (params (TouchedComponent :type "PrimitiveComponent Object Reference") (ButtonPressed :type "Key Structure"))
  (bind _outactors (`GameplayStatics.GetAllActorsWithInterface` "/Game/Blueprints/NPC_Interaction.NPC_Interaction_C"))
  (for _array_element _outactors
    (message `/Game/Blueprints/NPC_Interaction.NPCTalking` _array_element self)))

(event `/Game/Blueprints/NPC_Interaction.NPCNamePlates`
  (params (NPC :type "/Game/Blueprints/BaseChar_BP Object Reference") (`On/Off` :type Boolean))
  (`SceneComponent.SetVisibility` (`/Game/Blueprints/BaseChar_BP.Nameplate` NPC) `On/Off` false))

(fn `UserConstructionScript`
  (`parent.UserConstructionScript`))