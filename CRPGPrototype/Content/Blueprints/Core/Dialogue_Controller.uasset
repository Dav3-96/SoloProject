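; Dialogue controller that opens a conversation window when the player is close enough to a chosen NPC.
; NPCTalking checks the player's distance to the NPC and, when out of range, re-checks through a looping timer whose handle lives on the player controller.
; In range, it clears that timer, sets the controller's GamePaused flag and creates the DialogueWindow from the NPC's conversation and response data.
; The NPC's ground circle material switches with the range state.
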(event `self.ReceiveBeginPlay`
  (set `self.PlayerCharacter` (cast `/Game/Blueprints/BaseChar_BP` (`Controller.K2_GetPawn` (`GameplayStatics.GetPlayerController` 0)) :!pure true))
  (set `self.PlayerController` (cast `/Game/Blueprints/BP_PlayerController` (`GameplayStatics.GetPlayerController` 0) :!pure true)))

(event `self.NPCTalking`
  (params (NPC :type "/Game/Blueprints/NPC_BP Object Reference"))
  (bind _npc (`self.NPC`))
  (bind _playercontroller (`self.PlayerController`))
  (bind _player_responses_dialogue (break `/Game/Blueprints/Dialogues/Player_TotalConversation` (`/Game/Blueprints/NPC_BP.Player_Responses` _npc)))
  (bind (_npc_conversations_npcname _npc_conversations_dialogue) (break `/Game/Blueprints/Dialogues/NPC_TotalConveration` (`/Game/Blueprints/NPC_BP.NPC_Conversations` _npc)))
  (set `self.NPC` NPC)
  (if (<= (`self.GetDistanceTo` (`self.NPC`) (`self.PlayerCharacter`)) 150.0)
    (`KismetSystemLibrary.K2_ClearAndInvalidateTimerHandle` (`/Game/Blueprints/BP_PlayerController.DialogueInitiateTimer` (`self.PlayerController`)))
    (`PrimitiveComponent.SetMaterial` (`/Game/Blueprints/BaseChar_BP.GroundCircle` (`self.NPC`)) 0 "/Game/Mats/M_GroundCircle.M_GroundCircle")
    (set `/Game/Blueprints/BP_PlayerController.GamePaused` true _playercontroller)
    (bind _returnvalue (`|CreateWidget` "/Game/Blueprints/UI/DialogueWindow.DialogueWindow_C" _playercontroller null _npc_conversations_npcname (`/Game/Blueprints/NPC_BP.Has Responses?` _npc) _npc_conversations_dialogue _player_responses_dialogue))
    (`UserWidget.AddToViewport` _returnvalue 0)
    (else
      (bind _returnvalue_2 (`KismetSystemLibrary.K2_SetTimerDelegate` (delegate `MovingToRange`) 0.1 true))
      (set `/Game/Blueprints/BP_PlayerController.DialogueInitiateTimer` _returnvalue_2 (`self.PlayerController`))
      (`PrimitiveComponent.SetMaterial` (`/Game/Blueprints/BaseChar_BP.GroundCircle` (`self.NPC`)) 0 "/Game/Decals/M_FloorMarker.M_FloorMarker"))))

(event `MovingToRange`
  (`self.NPCTalking` (`self.NPC`)))

(fn `UserConstructionScript`)