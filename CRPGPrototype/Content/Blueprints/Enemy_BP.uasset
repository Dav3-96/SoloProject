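; Enemy NPC Blueprint with a floating nameplate, clickable for attack and fighting back with d20-style combat rolls.
; Clicking notifies NPC_Interaction actors; taking damage targets the causing player, updates health and starts a looping attack timer once.
; Attacks move toward distant players or roll in range, logging to combat UI; natural 20s log double damage and shake the camera.
; At zero health it ragdolls, then is destroyed.
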(event `/Game/Blueprints/NPC_Interaction.NPCNamePlates`
  (params (NPC :type "/Game/Blueprints/BaseChar_BP Object Reference") (`On/Off` :type Boolean))
  (`SceneComponent.SetVisibility` (`/Game/Blueprints/BaseChar_BP.Nameplate` NPC) `On/Off` false))

(event `self.ReceiveBeginPlay`
  (bind _asenemy_floating_names (cast `/Game/Blueprints/UI/EnemyFloatingNames` (`WidgetComponent.GetWidget` (`self.Nameplate`)) :!pure true))
  (set `/Game/Blueprints/UI/EnemyFloatingNames.NPC` self _asenemy_floating_names)
  (set `self.EnemyFloatingNameRef` _asenemy_floating_names))

(event `self.CapsuleComponent.OnClicked`
  (params (TouchedComponent :type "PrimitiveComponent Object Reference") (ButtonPressed :type "Key Structure"))
  (bind _outactors (`GameplayStatics.GetAllActorsWithInterface` "/Game/Blueprints/NPC_Interaction.NPC_Interaction_C"))
  (for _array_element _outactors
    (message `/Game/Blueprints/NPC_Interaction.AttackEnemy` _array_element self)))

(event `self.ReceiveAnyDamage`
  (params (Damage :type "Float (single-precision)") (DamageType :type "DamageType Object Reference") (InstigatedBy :type "Controller Object Reference") (DamageCauser :type "Actor Object Reference"))
  (bind _output_get (set `self.NPC_Health` (`KismetMathLibrary.FTrunc` (- (`self.NPC_Health`) Damage))))
  (bind _output_get_2 (set `self.PlayerCharacter` (cast `/Game/Blueprints/PC_Character` DamageCauser :!pure true)))
  (set `self.NPC_Target` _output_get_2)
  (`/Game/Blueprints/UI/EnemyFloatingNames.UpdateNameplateHeath` (`self.EnemyFloatingNameRef`))
  (`|ExecutionSequence`
    (:`then_0`
      (`/Engine/EditorBlueprintResources/StandardMacros.DoOnce` false
        (:`Completed`
          (`self.Fighting`))))
    (:`then_1`
      (if (<= _output_get 0)
        (`PrimitiveComponent.SetSimulatePhysics` (`self.Mesh`) true)
        (`KismetSystemLibrary.K2_ClearAndInvalidateTimerHandle` (`self.NPC_FightingTimer`))
        (`KismetSystemLibrary.Delay` 4.0)
        (`self.K2_DestroyActor`)))))

(event `Fighting`
  (bind _returnvalue (`KismetSystemLibrary.K2_SetTimerDelegate` (delegate `Attack`) (`self.NPC_ActionSpeed`) true))
  (set `self.NPC_FightingTimer` _returnvalue))

(event `Attack`
  (if (<= (`self.GetDistanceTo` self (`self.PlayerCharacter`)) 150.0)
    (`KismetSystemLibrary.K2_ClearAndInvalidateTimerHandle` (`self.EnemyMoveToAttack_Timer`))
    (set `self.NPC_HitRoll` (`KismetMathLibrary.RandomIntegerInRange` 1 20))
    (set `self.NPC_DamageRoll` (`KismetMathLibrary.RandomIntegerInRange` (`self.NPC_MinDamage`) (`self.NPC_MaxDamage`)))
    (if (>= (+ (`self.NPC_HitRoll`) (`self.BonusToHit`)) 0)
      (if (== (`self.NPC_HitRoll`) 20)
        (`/Game/Blueprints/UI/CombatInformation.SpawnEnemyCombatLogText` (`/Game/Blueprints/UI/CoreGame_UI.CombatInformation` (`/Game/Blueprints/BP_PlayerController.InGameUI` (cast `/Game/Blueprints/BP_PlayerController` (`GameplayStatics.GetPlayerController` 0) :!pure true))) (`self.NPC_Target`) self (* (`self.NPC_DamageRoll`) 2) false (`self.NPC_HitRoll`) (`/Game/Blueprints/PC_Character.ArmourClass` (`self.NPC_Target`)) true)
        (`self.DamageTarget`)
        (else
          (`/Game/Blueprints/UI/CombatInformation.SpawnEnemyCombatLogText` (`/Game/Blueprints/UI/CoreGame_UI.CombatInformation` (`/Game/Blueprints/BP_PlayerController.InGameUI` (cast `/Game/Blueprints/BP_PlayerController` (`GameplayStatics.GetPlayerController` 0) :!pure true))) (`self.NPC_Target`) self (`self.NPC_DamageRoll`) false (`self.NPC_HitRoll`) (`/Game/Blueprints/PC_Character.ArmourClass` (`self.NPC_Target`)) false)
          (`self.DamageTarget`)))
      (else
        (`/Game/Blueprints/UI/CombatInformation.SpawnEnemyCombatLogText` (`/Game/Blueprints/UI/CoreGame_UI.CombatInformation` (`/Game/Blueprints/BP_PlayerController.InGameUI` (cast `/Game/Blueprints/BP_PlayerController` (`GameplayStatics.GetPlayerController` 0) :!pure true))) (`self.NPC_Target`) self (`self.NPC_DamageRoll`) true (`self.NPC_HitRoll`) (`/Game/Blueprints/PC_Character.ArmourClass` (`self.NPC_Target`)) false)))
    (else
      (bind _returnvalue (`KismetSystemLibrary.K2_SetTimerDelegate` (delegate `Check For Range`) 0.1))
      (set `self.EnemyMoveToAttack_Timer` _returnvalue))))

(event `Check For Range`
  (`AIBlueprintHelperLibrary.SimpleMoveToActor` (`self.GetController`) (`self.PlayerCharacter`)))

(fn `DamageTarget`
  (`GameplayStatics.ApplyDamage` (`self.NPC_Target`) (`KismetMathLibrary.Conv_IntToDouble` (`self.NPC_DamageRoll`)) null self)
  (if (== (`self.NPC_HitRoll`) 20)
    (`GameplayStatics.PlayWorldCameraShake` "/Game/Blueprints/CameraShaker.CameraShaker_C" (`self.K2_GetActorLocation` (`self.NPC_Target`)) 0.0 100000.0))
  (if (<= (`/Game/Blueprints/BaseChar_BP.Health` (`self.NPC_Target`)) 0)
    (`KismetSystemLibrary.K2_ClearAndInvalidateTimerHandle` (`self.NPC_FightingTimer`))))

(fn `UserConstructionScript`
  (`parent.UserConstructionScript`)
  (setmembers `/Game/Blueprints/Enemies/NPC_Stats` :`StructRef` (`self.NPC_Stats`) :`DamageMin` (`self.NPC_MinDamage`) :`DamageMax` (`self.NPC_MaxDamage`) :`ActionSpeed` (`self.NPC_ActionSpeed`) :`Health` (`self.NPC_Health`) :`ArmourClass` (`self.NPC_ArmourClass`) :`Name` (`self.Name`)))