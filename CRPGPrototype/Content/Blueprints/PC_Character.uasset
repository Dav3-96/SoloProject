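; Player character Blueprint for dice-based combat, copying its stats from the Master_Instance game instance on BeginPlay.
; Fighting starts a looping timer that rolls d20 plus bonus against the target's armour class, logging results to the UI.
; Natural 20s that hit log doubled damage and shake the camera, but DamageTarget applies the undoubled roll, stopping the timer at zero target health.
; Damage taken updates the health UI and ragdolls the mesh at zero.
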(event `self.ReceiveBeginPlay`
  (set `self.As Master Instance` (cast `/Game/Blueprints/Character_Info/Master_Instance` (`GameplayStatics.GetGameInstance`) :!pure true))
  (set `self.PlayerController` (cast `/Game/Blueprints/BP_PlayerController` (`self.GetController`) :!pure true))
  (`self.InitCharacter`))

(event `self.ReceiveTick`
  (params (DeltaSeconds :type "Float (single-precision)")))

(event `self.ReceiveAnyDamage`
  (params (Damage :type "Float (single-precision)") (DamageType :type "DamageType Object Reference") (InstigatedBy :type "Controller Object Reference") (DamageCauser :type "Actor Object Reference"))
  (bind _output_get (set `self.Health` (`KismetMathLibrary.FTrunc` (- (`self.Health`) Damage))))
  (`/Game/Blueprints/UI/CharacterCreation/CharacterImages_UI.UpdateHealth` (`/Game/Blueprints/UI/CoreGame_UI.CharacterImages_UI` (`/Game/Blueprints/BP_PlayerController.InGameUI` (`self.PlayerController`))) _output_get (`self.MaxHealth`))
  (`|ExecutionSequence`
    (:`then_1`
      (if (<= _output_get 0)
        (`PrimitiveComponent.SetSimulatePhysics` (`self.Mesh`) true)))))

(event `InitCharacter`
  (set `self.Health` (`/Game/Blueprints/Character_Info/Master_Instance.Health` (`self.As Master Instance`)))
  (set `self.MaxHealth` (`/Game/Blueprints/Character_Info/Master_Instance.MaxHealth` (`self.As Master Instance`)))
  (set `self.DamageMin` (`/Game/Blueprints/Character_Info/Master_Instance.DamageMin` (`self.As Master Instance`)))
  (set `self.DamageMax` (`/Game/Blueprints/Character_Info/Master_Instance.DamageMax` (`self.As Master Instance`)))
  (set `self.ActionSpeed` (`/Game/Blueprints/Character_Info/Master_Instance.Action Speed` (`self.As Master Instance`)))
  (set `self.ArmourClass` (`/Game/Blueprints/Character_Info/Master_Instance.ArmourClass` (`self.As Master Instance`)))
  (set `self.CharName` (`/Game/Blueprints/Character_Info/Master_Instance.CharName` (`self.As Master Instance`))))

(event `Fighting`
  (bind _returnvalue (`KismetSystemLibrary.K2_SetTimerDelegate` (delegate `Attack`) (`self.ActionSpeed`) true))
  (set `self.FightingTimer` _returnvalue)
  (set `/Game/Blueprints/BP_PlayerController.MovementStates` "NewEnumerator3" (`self.PlayerController`)))

(event `Attack`
  (bind _npc_armourclass (`/Game/Blueprints/Enemy_BP.NPC_ArmourClass` (`self.Target`)))
  (set `self.HitRoll` (`KismetMathLibrary.RandomIntegerInRange` 1 20))
  (set `self.DamageRoll` (`KismetMathLibrary.RandomIntegerInRange` (`self.DamageMin`) (`self.DamageMax`)))
  (if (>= (+ (`self.HitRoll`) (`self.BonusToHit`)) _npc_armourclass)
    (if (== (`self.HitRoll`) 20)
      (`/Game/Blueprints/UI/Combat/CombatInformation.SpawnPlayerCombatLogText` (`/Game/Blueprints/UI/CoreGame_UI.CombatInformation` (`/Game/Blueprints/BP_PlayerController.InGameUI` (`self.PlayerController`))) (`self.Target`) self (* (`self.DamageRoll`) 2) false (`self.HitRoll`) (`/Game/Blueprints/Enemy_BP.NPC_ArmourClass` (`self.Target`)) true)
      (`self.DamageTarget`)
      (else
        (`/Game/Blueprints/UI/Combat/CombatInformation.SpawnPlayerCombatLogText` (`/Game/Blueprints/UI/CoreGame_UI.CombatInformation` (`/Game/Blueprints/BP_PlayerController.InGameUI` (`self.PlayerController`))) (`self.Target`) self (`self.DamageRoll`) false (`self.HitRoll`) (`/Game/Blueprints/Enemy_BP.NPC_ArmourClass` (`self.Target`)) false)
        (`self.DamageTarget`)))
    (else
      (`/Game/Blueprints/UI/Combat/CombatInformation.SpawnPlayerCombatLogText` (`/Game/Blueprints/UI/CoreGame_UI.CombatInformation` (`/Game/Blueprints/BP_PlayerController.InGameUI` (`self.PlayerController`))) (`self.Target`) self (`self.DamageRoll`) true (`self.HitRoll`) _npc_armourclass false))))

(fn `DamageTarget`
  (`GameplayStatics.ApplyDamage` (`self.Target`) (`KismetMathLibrary.Conv_IntToDouble` (`self.DamageRoll`)) null self)
  (if (== (`self.HitRoll`) 20)
    (`GameplayStatics.PlayWorldCameraShake` "/Game/Blueprints/CameraShaker.CameraShaker_C" (`self.K2_GetActorLocation` (`self.Target`)) 0.0 100000.0))
  (if (<= (`/Game/Blueprints/Enemy_BP.NPC_Health` (`self.Target`)) 0)
    (`KismetSystemLibrary.K2_ClearAndInvalidateTimerHandle` (`self.FightingTimer`))))

(fn `UserConstructionScript`
  (`parent.UserConstructionScript`))