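; Master instance that holds the player character's stats, skills, choices and derived values, and saves and loads them through Save_SaveGame.
; Save and Load use one fixed slot, with a helper per data group; Load falls back to a new save object.
; Loading location opens the saved level if different, then immediately repositions the player.
; RunStatCalc derives combat and vendor values from base stats and modifiers, separately from loading.
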(event `Save`
  (`/Engine/EditorBlueprintResources/StandardMacros.IsValid` (`self.SaveGame`)
    (:`Is Valid`
      _)
    (:`Is Not Valid`
      (bind _returnvalue (`GameplayStatics.CreateSaveGameObject` "/Game/Blueprints/Saves/Save_SaveGame.Save_SaveGame_C"))
      (set `self.SaveGame` _returnvalue)))
  (`self.SaveLocation`)
  (`self.SaveStats`)
  (`self.SaveSkills`)
  (`self.SaveChoices`)
  (`self.SaveModifiers`)
  (`self.SaveCurrentValues`)
  (`GameplayStatics.SaveGameToSlot` (`self.SaveGame`) "savegame"))

(event `Load`
  (bind _returnvalue (`GameplayStatics.DoesSaveGameExist` "savegame"))
  (if _returnvalue
    (bind _returnvalue_2 (`GameplayStatics.LoadGameFromSlot` "savegame"))
    (bind _assave_save_game (cast `/Game/Blueprints/Saves/Save_SaveGame` _returnvalue_2))
    (set `self.SaveGame` _assave_save_game)
    (else
      (bind _returnvalue_3 (`GameplayStatics.CreateSaveGameObject` "/Game/Blueprints/Saves/Save_SaveGame.Save_SaveGame_C"))
      (set `self.SaveGame` _returnvalue_3)))
  (`self.Load Location`)
  (`self.Load Stats`)
  (`self.Load Skills`)
  (`self.Load Choices`)
  (`self.LoadModifiers`)
  (`self.LoadCurrentValues`))

(event `StrCalc`
  (bind _output_get (set `self.BaseStrength` (/ (+ (`self.BaseStrength`) (`self.StrengthMod`)) 8)))
  (bind _returnvalue (`KismetMathLibrary.Conv_IntToDouble` _output_get))
  (set `self.DamageMin` (`KismetMathLibrary.Round` (* _returnvalue 0.2)))
  (set `self.DamageMax` (`KismetMathLibrary.Round` (* _returnvalue 0.8))))

(event `ConCalc`
  (bind _output_get (set `self.BaseConstitution` (/ (+ (`self.BaseConstitution`) (`self.ConstitutionMod`)) 8)))
  (bind _output_get_2 (set `self.Health` (`KismetMathLibrary.Round` (* (`KismetMathLibrary.Conv_IntToDouble` _output_get) (`self.HPLevelMulti`)))))
  (set `self.MaxHealth` _output_get_2))

(event `DexCalc`
  (set `self.Action Speed` (/ (`KismetMathLibrary.Conv_IntToDouble` (+ (`self.BaseDexterity`) (`self.DexterityMod`))) 100.0)))

(event `IntCalc`
  (set `self.Spell Damage` (`self.IntellectMod`)))

(event `WisCalc`
  (set `self.Spell Healing` (`self.WisdomMod`)))

(event `ChaCalc`
  (set `self.Vendor Price` (`self.CharismaMod`)))

(fn `Load Choices`
  (bind (_race _gender _class _portrait _name) (break `/Game/Blueprints/Saves/S_SavePlayerChoices` (`/Game/Blueprints/Saves/Save_SaveGame.PlayerChoices` (`self.SaveGame`))))
  (set `self.Race` _race)
  (set `self.Gender` _gender)
  (set `self.Class` _class)
  (set `self.PlayerImage` _portrait)
  (set `self.CharName` _name))

(fn `Load Location`
  (bind _currentlevel (`/Game/Blueprints/Saves/Save_SaveGame.CurrentLevel` (`self.SaveGame`)))
  (`|ExecutionSequence`
    (:`then_0`
      (bind _returnvalue (`GameplayStatics.GetCurrentLevelName` true))
      (if (not (== _currentlevel _returnvalue))
        (`GameplayStatics.OpenLevel` _currentlevel true "game=InGame")))
    (:`then_1`
      (`Actor.K2_SetActorLocation` (`GameplayStatics.GetPlayerCharacter` 0) (`/Game/Blueprints/Saves/Save_SaveGame.PlayerPosition` (`self.SaveGame`)) false false))))

(fn `Load Skills`
  (bind (_athletics _survival _stealth _thievery _religion _nature _arcana) (break `/Game/Blueprints/Saves/S_SavePlayerSkills` (`/Game/Blueprints/Saves/Save_SaveGame.PlayerSkills` (`self.SaveGame`))))
  (set `self.Athletics` _athletics)
  (set `self.Survival` _survival)
  (set `self.Stealth` _stealth)
  (set `self.Thivery` _thievery)
  (set `self.Religion` _religion)
  (set `self.Nature` _nature)
  (set `self.Arcana` _arcana))

(fn `Load Stats`
  (bind (_strength _dexterity _constitution _intelligence _wisdom _charisma) (break `/Game/Blueprints/Saves/S_SavePlayerStats` (`/Game/Blueprints/Saves/Save_SaveGame.PlayerStats` (`self.SaveGame`))))
  (set `self.Strength` _strength)
  (set `self.Dexterity` _dexterity)
  (set `self.Constitution` _constitution)
  (set `self.Intelligence` _intelligence)
  (set `self.Wisdom` _wisdom)
  (set `self.Charisma` _charisma))

(fn `LoadCurrentValues`
  (bind (_health _maxhealth _attackspeed _armorclass _damagemin _damagemax _spelldamage _spellhealing _vendorprice) (break `/Game/Blueprints/Saves/S_SavePlayerValues` (`/Game/Blueprints/Saves/Save_SaveGame.PlayerValues` (`self.SaveGame`))))
  (set `self.Health` _health)
  (set `self.MaxHealth` _maxhealth)
  (set `self.Action Speed` _attackspeed)
  (set `self.ArmourClass` _armorclass)
  (set `self.DamageMin` _damagemin)
  (set `self.DamageMax` _damagemax)
  (set `self.Spell Damage` _spelldamage)
  (set `self.Spell Healing` _spellhealing)
  (set `self.Vendor Price` _vendorprice))

(fn `LoadModifiers`
  (bind (_strmod _dexmod _conmod _intmod _wismod _chamod) (break `/Game/Blueprints/Saves/S_SaveStatModifiers` (`/Game/Blueprints/Saves/Save_SaveGame.PlayerStatMod` (`self.SaveGame`))))
  (set `self.StrengthMod` _strmod)
  (set `self.DexterityMod` _dexmod)
  (set `self.ConstitutionMod` _conmod)
  (set `self.IntellectMod` _intmod)
  (set `self.WisdomMod` _wismod)
  (set `self.CharismaMod` _chamod))

(fn `RunStatCalc`
  (`self.StrCalc`)
  (`self.DexCalc`)
  (`self.ConCalc`)
  (`self.IntCalc`)
  (`self.WisCalc`)
  (`self.ChaCalc`))

(fn `SaveChoices`
  (setmembers `/Game/Blueprints/Saves/S_SavePlayerChoices` :`StructRef` (`/Game/Blueprints/Saves/Save_SaveGame.PlayerChoices` (`self.SaveGame`)) :`Race` (`self.Race`) :`Gender` (`self.Gender`) :`Class` (`self.Class`) :`Portrait` (`self.PlayerImage`) :`Name` (`self.CharName`)))

(fn `SaveCurrentValues`
  (setmembers `/Game/Blueprints/Saves/S_SavePlayerValues` :`StructRef` (`/Game/Blueprints/Saves/Save_SaveGame.PlayerValues` (`self.SaveGame`)) :`Health` (`self.Health`) :`MaxHealth` (`self.MaxHealth`) :`Attack Speed` (`self.Action Speed`) :`ArmorClass` (`self.ArmourClass`) :`DamageMin` (`self.DamageMin`) :`DamageMax` (`self.DamageMax`) :`SpellDamage` (`self.Spell Damage`) :`SpellHealing` (`self.Spell Healing`) :`VendorPrice` (`self.Vendor Price`)))

(fn `SaveLocation`
  (bind _returnvalue (`GameplayStatics.GetCurrentLevelName` true))
  (set `/Game/Blueprints/Saves/Save_SaveGame.CurrentLevel` (`KismetStringLibrary.Conv_StringToName` _returnvalue) (`self.SaveGame`))
  (set `/Game/Blueprints/Saves/Save_SaveGame.PlayerPosition` (`Actor.K2_GetActorLocation` (`GameplayStatics.GetPlayerCharacter` 0)) (`self.SaveGame`)))

(fn `SaveModifiers`
  (setmembers `/Game/Blueprints/Saves/S_SaveStatModifiers` :`StructRef` (`/Game/Blueprints/Saves/Save_SaveGame.PlayerStatMod` (`self.SaveGame`)) :`StrMod` (`self.StrengthMod`) :`DexMod` (`self.DexterityMod`) :`ConMod` (`self.ConstitutionMod`) :`IntMod` (`self.IntellectMod`) :`WisMod` (`self.WisdomMod`) :`ChaMod` (`self.CharismaMod`)))

(fn `SaveSkills`
  (setmembers `/Game/Blueprints/Saves/S_SavePlayerSkills` :`StructRef` (`/Game/Blueprints/Saves/Save_SaveGame.PlayerSkills` (`self.SaveGame`)) :`Athletics` (`self.Athletics`) :`Survival` (`self.Survival`) :`Stealth` (`self.Stealth`) :`Thievery` (`self.Thivery`) :`Religion` (`self.Religion`) :`Nature` (`self.Nature`) :`Arcana` (`self.Arcana`)))

(fn `SaveStats`
  (setmembers `/Game/Blueprints/Saves/S_SavePlayerStats` :`StructRef` (`/Game/Blueprints/Saves/Save_SaveGame.PlayerStats` (`self.SaveGame`)) :`Strength` (`self.Strength`) :`Dexterity` (`self.Dexterity`) :`Constitution` (`self.Constitution`) :`Intelligence` (`self.Intelligence`) :`Wisdom` (`self.Wisdom`) :`Charisma` (`self.Charisma`)))