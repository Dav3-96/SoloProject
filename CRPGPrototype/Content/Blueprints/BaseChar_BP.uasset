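; BaseChar_BP is a character Blueprint, apparently a base class, that color-codes characters as friendly, enemy or NPC.
; Its construction script writes DepthColour as the custom depth stencil value on both the Mesh and the GroundCircle.
; The same value selects the matching ground indicator material, applied to GroundCircle as a dynamic instance through a switch flagged in the graph as needing cleanup.
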(fn `UserConstructionScript`
  (bind _depthcolour (`self.DepthColour`))
  (`PrimitiveComponent.SetCustomDepthStencilValue` (`self.Mesh`) (`self.DepthColour`))
  (`PrimitiveComponent.SetCustomDepthStencilValue` (`self.GroundCircle`) _depthcolour)
  (switch `int` _depthcolour
    (:`1`
      ;[1 1 1] NEEDS FIXING - THIS IS MESSY
      (`PrimitiveComponent.CreateDynamicMaterialInstance` (`self.GroundCircle`) 0 "/Game/Mats/MI_GroundIndicatorFriendly.MI_GroundIndicatorFriendly" "None"))
    (:`2`
      (`PrimitiveComponent.CreateDynamicMaterialInstance` (`self.GroundCircle`) 0 "/Game/Mats/MI_GroundIndicatorEnemy.MI_GroundIndicatorEnemy" "None"))
    (:`3`
      (`PrimitiveComponent.CreateDynamicMaterialInstance` (`self.GroundCircle`) 0 "/Game/Mats/MI_GroundIndicatorNPC.MI_GroundIndicatorNPC" "None"))))