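; Talkable NPC that starts a dialogue once the player character is close enough.
; On BeginPlay it caches the player character and controller, then hands its DialogueTree to its AIC_NPC controller.
; Interact registers the NPC on the player controller and polls distance with a looping timer until in range, then clears it and calls StartDialogue on the AI controller.
; The logic setting the FloatingNames widget's character name is disconnected.
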(event `self.ReceiveBeginPlay`
  (bind _returnvalue (`GameplayStatics.GetActorOfClass` "/Game/Blueprints/PC_Character.PC_Character_C"))
  (set `self.Character` _returnvalue)
  (set `self.PlayerController` (cast `/Game/Blueprints/BP_PlayerController` (`GameplayStatics.GetPlayerController` 0) :!pure true))
  (bind _asaic_npc (cast `/Game/Blueprints/NPC/AI/AIC_NPC` (`AIBlueprintHelperLibrary.GetAIController` self)))
  (set `/Game/Blueprints/NPC/AI/AIC_NPC.DialogueTree` (`self.DialogueTree`) _asaic_npc))

(event `self.Interact`
  ;[1 1 1] Constantly checks for player in range
  (set `/Game/Blueprints/BP_PlayerController.NPCReference` self (`self.PlayerController`))
  (if (<= (`self.GetDistanceTo` (`self.Character`)) 250.0)
    (`KismetSystemLibrary.K2_ClearAndInvalidateTimerHandle` (`self.PlayerMovingToActor`))
    (`/Game/Blueprints/NPC/AI/AIC_NPC.StartDialogue` (cast `/Game/Blueprints/NPC/AI/AIC_NPC` (`AIBlueprintHelperLibrary.GetAIController` self) :!pure true))
    (else
      (bind _returnvalue (`KismetSystemLibrary.K2_SetTimerDelegate` (delegate `MovingToActor`) 0.1 true))
      (set `self.PlayerMovingToActor` _returnvalue))))

(event `MovingToActor`
  ;[1 1 1] Constantly checks for player in range
  (`self.Interact`))

(fn `UserConstructionScript`)