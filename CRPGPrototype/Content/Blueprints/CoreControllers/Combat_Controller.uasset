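; Combat controller Blueprint that starts and stops the player character's attacks on a target enemy.
; AttackEnemy sets the character's target, then calls Fighting if the enemy is within melee range.
; Otherwise it applies a floor-marker material to the enemy's ground circle and re-checks range on a looping timer stored on the player controller.
; StopAttack clears only the character's fighting timer, leaving the range-check timer untouched.
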(event `self.ReceiveBeginPlay`
  (set `self.PlayerCharacter` (cast `/Game/Blueprints/PC_Character` (`Controller.K2_GetPawn` (`GameplayStatics.GetPlayerController` 0)) :!pure true))
  (set `self.PlayerController` (cast `/Game/Blueprints/BP_PlayerController` (`GameplayStatics.GetPlayerController` 0) :!pure true)))

(event `self.AttackEnemy`
  (params (Enemy :type "/Game/Blueprints/Enemy_BP Object Reference"))
  (bind _output_get (set `self.Enemy` Enemy))
  (set `/Game/Blueprints/PC_Character.Target` _output_get (`self.PlayerCharacter`))
  (if (<= (`self.GetDistanceTo` (`self.Enemy`) (`self.PlayerCharacter`)) 150.0)
    (`KismetSystemLibrary.K2_ClearAndInvalidateTimerHandle` (`/Game/Blueprints/BP_PlayerController.MoveToAttackTimer` (`self.PlayerController`)))
    (`/Game/Blueprints/PC_Character.Fighting` (`self.PlayerCharacter`))
    (else
      (bind _returnvalue (`KismetSystemLibrary.K2_SetTimerDelegate` (delegate `MovingToRange`) 0.1 true))
      (set `/Game/Blueprints/BP_PlayerController.MoveToAttackTimer` _returnvalue (`self.PlayerController`))
      (`PrimitiveComponent.SetMaterial` (`/Game/Blueprints/BaseChar_BP.GroundCircle` (`self.Enemy`)) 0 "/Game/Decals/M_FloorMarker.M_FloorMarker"))))

(event `MovingToRange`
  (`self.AttackEnemy` (`self.Enemy`)))

(event `self.StopAttack`
  (bind _fightingtimer (`/Game/Blueprints/PC_Character.FightingTimer` (`self.PlayerCharacter`)))
  (if (`KismetSystemLibrary.K2_IsValidTimerHandle` _fightingtimer)
    (`KismetSystemLibrary.K2_ClearAndInvalidateTimerHandle` _fightingtimer)))

(fn `UserConstructionScript`)