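; Floating damage number actor that shows a hit's damage on a widget component and removes itself.
; On BeginPlay it destroys itself at once if the hit missed.
; Otherwise it passes damage and critical-hit state to its FloatingDamageNumbers widget, then destroys itself after a short delay.
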(event `self.ReceiveBeginPlay`
  (if (`self.Missed?`)
    (`self.K2_DestroyActor`)
    (else
      (bind _asfloating_damage_numbers (cast `/Game/Blueprints/UI/Combat/FloatingDamageNumbers` (`WidgetComponent.GetUserWidgetObject` (`self.FloatingDamage`))))
      (`/Game/Blueprints/UI/Combat/FloatingDamageNumbers.SetupText` _asfloating_damage_numbers (`self.Damage`) (`self.CriticalHit?`))
      (`KismetSystemLibrary.Delay` 1.0)
      (`self.K2_DestroyActor`))))

(fn `UserConstructionScript`)