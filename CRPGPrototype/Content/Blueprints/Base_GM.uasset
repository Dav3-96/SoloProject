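; Base game mode that sets up the local player and in-game UI when play begins.
; BeginPlay caches the player controller and controlled character, sets game-and-UI input with the mouse locked, then starts an init chain.
; The chain loads through Master_Instance if Continue was pressed, then creates the CoreGame_UI widget and initializes it with the controller and character.
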(event `self.ReceiveBeginPlay`
  (bind _returnvalue (`GameplayStatics.GetPlayerController` 0))
  (set `self.PlayerController` (cast `/Game/Blueprints/BP_PlayerController` _returnvalue :!pure true))
  (set `self.PlayerCharacter` (cast `/Game/Blueprints/BaseChar_BP` (`Controller.K2_GetPawn` _returnvalue) :!pure true))
  (`WidgetBlueprintLibrary.SetInputMode_GameAndUIEx` (`self.PlayerController`) null "LockAlways" false)
  (`self.Begin_InitChain`))

(event `Begin_InitChain`
  (bind _asmaster_instance (cast `/Game/Blueprints/Character_Info/Master_Instance` (`GameplayStatics.GetGameInstance`)))
  (if (`/Game/Blueprints/Character_Info/Master_Instance.PressedContinue?` _asmaster_instance)
    (`/Game/Blueprints/Character_Info/Master_Instance.Load` _asmaster_instance))
  (bind _returnvalue (`|CreateWidget` "/Game/Blueprints/UI/CoreGame_UI.CoreGame_UI_C" (`self.PlayerController`)))
  (bind _output_get (set `self.InGameUI` _returnvalue))
  (`UserWidget.AddToViewport` _output_get 0)
  (`/Game/Blueprints/UI/CoreGame_UI.InGameUI_Init` _returnvalue (`self.PlayerController`) (cast `/Game/Blueprints/PC_Character` (`self.PlayerCharacter`) :!pure true)))

(fn `UserConstructionScript`)